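; BP_SlingShotRock is a rock actor, apparently the projectile for an enemy slingshot ability, that tumbles visually.
; BeginPlay picks random yaw, pitch and roll rates, each able to spin in either direction.
; Tick applies those rates to RockMesh as a delta-time-scaled local rotation.
; This graph contains only the cosmetic spin, with no movement, collision or damage logic.
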(event EventBeginPlay
  (bind _returnvalue (Math|Random|RandomFloatinRange -5e+02 5e+02))
  (Variables|Default|SetYawRotaionRate _returnvalue)
  (Variables|Default|SetPitchRotaionRate _returnvalue)
  (Variables|Default|SetRollRotaionRate _returnvalue))

(event Collision|EventActorBeginOverlap
  (params (OtherActor :type Actor%20Object%20Reference)))

(event EventTick
  (params (DeltaSeconds :type Float%20%28single-precision%29))
  (Transformation|AddLocalRotation (Variables|Default|GetRockMesh) (Math|Rotator|MakeRotator (* DeltaSeconds (Variables|Default|GetRollRotaionRate)) (* DeltaSeconds (Variables|Default|GetPitchRotaionRate)) (* DeltaSeconds (Variables|Default|GetYawRotaionRate))) false false))

(fn ConstructionScript)